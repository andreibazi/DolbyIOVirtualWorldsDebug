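; Debug actor that exercises the Dolby.io plugin's camera enumeration and switching.
; When its DolbyIOObserver requests a token, it sets an empty one and, once initialized, fetches and counts the video devices.
; A chain of async nodes enables the first camera, waits briefly, disables it and enables the second, printing status on screen.
; The first two device indices are used without checking how many were found.
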(event `self.DolbyIOObserver.OnTokenNeeded`
  (`DolbyIOSetToken.DolbyIOSetToken` ""
    (:`OnInitialized`
      (bind _devices (`DolbyIOGetVideoDevices.DolbyIOGetVideoDevices`)
        (:`OnVideoDevicesReceived`
          (`KismetSystemLibrary.PrintString` (`KismetStringLibrary.Concat_StrStr` "Found " (`KismetStringLibrary.Conv_IntToString` (`KismetArrayLibrary.Array_Length` _devices)) " video devices.") true true (struct :`G` 1.0 :`B` 0.380003 :`A` 1.0) 20.0 "devices")
          (bind _output (`|GetArrayItem` _devices))
          (`DolbyIOEnableVideo.DolbyIOEnableVideo` _output
            (:`OnVideoEnabled`
              (`KismetSystemLibrary.PrintString` (`KismetStringLibrary.Concat_StrStr` "Previewing " (`KismetTextLibrary.Conv_TextToString` (`.Name` (break `DolbyIOVideoDevice` _output))) ". Switching to the next camera in 5 seconds.") true true (struct :`G` 0.66 :`B` 1.0 :`A` 1.0) 20.0 "camera")
              (`KismetSystemLibrary.Delay` 5.0)
              (`DolbyIODisableVideo.DolbyIODisableVideo`
                (:`OnVideoDisabled`
                  (bind _output_2 (`|GetArrayItem` _devices 1))
                  (`DolbyIOEnableVideo.DolbyIOEnableVideo` _output_2
                    (:`OnVideoEnabled`
                      (`KismetSystemLibrary.PrintString` (`KismetStringLibrary.Concat_StrStr` "Previewing " (`KismetTextLibrary.Conv_TextToString` (`.Name` (break `DolbyIOVideoDevice` _output_2))) ".") true true (struct :`G` 0.66 :`B` 1.0 :`A` 1.0) 20.0 "camera"))))))))))))

(fn `UserConstructionScript`)